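; Food manager actor that runs the eating rounds of a day, then depletes hunger and loads the Kitchen level.
; Each round it gives every BP_Food actor a random mesh and attribute, and feeding or passing applies player status and advances.
; Food interaction events set the selection, with overlay materials highlighting it or items revealed by the metal detector.
; UseItem applies consumable effects such as skipping rounds or curing ailments, with timed messages in the UI.
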(event Custom|SetSelectedFood
  (params (FoodItem :type BP%20Food%20Object%20Reference))
  (CallFunction|SelectFood FoodItem))

(event Custom|BindEvents
  (for _array_element (Variables|Default|GetFoodSpawns)
    (EventDispatchers|BindEventtoOnFoodInteraction _array_element (delegate Custom|SetSelectedFood))))

(event Custom|FeedPlayer
  (bind _selectedfood (Variables|Default|GetSelectedFood))
  (Utilities|IsValid _selectedfood
    (:Is%20Valid
      (Default|EatFood (Variables|Default|GetPlayer) _selectedfood)
      (CallFunction|UpdateUI)
      (CallFunction|ProgressRound))
    (:Is%20Not%20Valid
      (Development|PrintString "No valid selected food."))))

(event Custom|PassRound
  (Default|PassRound (Variables|Default|GetPlayer))
  (CallFunction|ProgressRound))

(event Custom|UpdateUIItem
  (Utilities|FlowControl|Delay 5.0)
  (Variables|Default|SetUIMessage ""))

(event Custom|ProgressRound
  (if (< (Variables|Default|GetCurrentRound) (Variables|Default|GetRoundsCount))
    (Default|ApplyStatus (Variables|Default|GetPlayer))
    (Math|Integer|IncrementInt (Variables|Default|GetCurrentRound)
      (:%20%20
        (CallFunction|SpawnFood)))
    (else
      (Default|ApplyStatus (Variables|Default|GetPlayer))
      (CallFunction|ProgressDay))))

(event Custom|UpdateUI
  (Variables|Default|SetUIMessage (Variables|/Game/Blueprints/Player/BP_Player.BP_Player_C|GetNotifString (Variables|Default|GetPlayer)))
  (Utilities|FlowControl|Delay 5.0)
  (Variables|Default|SetUIMessage ""))

(event Custom|ProgressDay
  (Class|PlayerChar|DepleteHunger (Variables|Default|GetPlayer) 20)
  (Widget|RemovefromParent (Variables|Default|GetUI))
  (Class|GameManager|ProgressDay (Variables|Default|GetGameManager))
  (Game|OpenLevel(byName) "Kitchen"))

(event EventBeginPlay
  (CallFunction|InitializeFoodManager)
  (CallFunction|SpawnFood))

(fn ConstructionScript)

(fn SpawnFood
  (for _array_element (Variables|Default|GetFoodSpawns)
    (bind _mesh (CallFunction|GetRandomMesh))
    (Default|SetMesh _array_element _mesh)
    (bind _attribute (CallFunction|GetRandomAttribute))
    (Default|SetAttribute _array_element _attribute)
    (Rendering|Material|SetOverlayMaterial (Variables|/Game/Blueprints/Food/BP_Food.BP_Food_C|GetStaticMesh _array_element) 0 :!class /Script/Engine.MeshComponent)))

(fn GetRandomMesh
  (return (.OutItem (Utilities|Array|Random (Variables|Default|GetFoodMeshes)))))

(fn GetRandomAttribute
  (return (.OutItem (Utilities|Array|Random (Variables|Default|GetAttributes)))))

(fn InitializeFoodManager
  (Variables|Default|SetCurrentRound 0)
  (bind _returnvalue (UserInterface|CreateWidget "/Game/Blueprints/UI/UI_Eating.UI_Eating_C"))
  (bind _output_get (Variables|Default|SetUI _returnvalue))
  (UserInterface|Viewport|AddtoViewport _output_get 0)
  (bind _returnvalue_2 (Actor|GetActorOfClass "/Game/Blueprints/Player/BP_Player.BP_Player_C"))
  (Variables|Default|SetPlayer _returnvalue_2)
  (bind _outactors (Actor|GetAllActorsOfClass "/Game/Blueprints/Food/BP_Food.BP_Food_C"))
  (Variables|Default|SetFoodSpawns _outactors)
  (bind _asgame_manager (Utilities|Casting|CastToGameManager (Game|GetGameInstance))
    (:then
      (bind _output_get_2 (Variables|Default|SetGameManager _asgame_manager))
      (bind _returnvalue_3 (Class|GameManager|GetRoundsCount _output_get_2))
      (Variables|Default|SetRoundsCount _returnvalue_3))
    (:CastFailed
      (Development|PrintString "Casting to GM failed.")))
  (CallFunction|BindEvents))

(fn MilkRound
  (CallFunction|ProgressRound))

(fn DetectAttribute
  (params (Attribute :type FoodAttribute%20Enum :default "NewEnumerator0"))
  (for _array_element (Variables|Default|GetFoodSpawns)
    (if (Utilities|Enum|Equal(Enum) (Variables|/Game/Blueprints/Food/BP_Food.BP_Food_C|GetAttribute _array_element) Attribute)
      (Rendering|Material|SetOverlayMaterial (Variables|/Game/Blueprints/Food/BP_Food.BP_Food_C|GetStaticMesh _array_element) "/Game/Assets/Materials/VFX/Mat_RedHighlight.Mat_RedHighlight" :!class /Script/Engine.MeshComponent))))

(fn SelectFood
  (params (SelectedFood :type BP%20Food%20Object%20Reference))
  (Utilities|IsValid (Variables|Default|GetSelectedFood)
    (:Is%20Valid
      (Rendering|Material|SetOverlayMaterial (Variables|/Game/Blueprints/Food/BP_Food.BP_Food_C|GetStaticMesh (Variables|Default|GetSelectedFood)) 0 :!class /Script/Engine.MeshComponent))
    (:Is%20Not%20Valid
      _))
  (bind _output_get (Variables|Default|SetSelectedFood SelectedFood))
  (Rendering|Material|SetOverlayMaterial (Variables|/Game/Blueprints/Food/BP_Food.BP_Food_C|GetStaticMesh _output_get) "/Game/Assets/Materials/VFX/Mat_BlueHighlight.Mat_BlueHighlight" :!class /Script/Engine.MeshComponent))

(fn UseItem
  (params (ItemType :type EItemType%20Enum :default "Milk"))
  (bind _player (Variables|Default|GetPlayer))
  (switch Utilities|FlowControl|Switch|SwitchonEItemType ItemType
    (:Milk
      (CallFunction|MilkRound)
      (Variables|Default|SetUIMessage "The milk fills your stomach with warmth"))
    (:MetalDetector
      (CallFunction|DetectAttribute "NewEnumerator4")
      (Variables|Default|SetUIMessage "The metal detector reveals hidden traps"))
    (:Antidote
      (Variables|/Game/Blueprints/Player/BP_Player.BP_Player_C|SetPoisonCounter _player 0)
      (Variables|Default|SetUIMessage "The antidote cures your poisoned blood"))
    (:Antacid
      (Variables|/Game/Blueprints/Player/BP_Player.BP_Player_C|SetTakenAntacid _player true)
      (Variables|Default|SetUIMessage "The antacid sets your stomach at ease"))
    (:Medicine
      (Class|PlayerChar|RestoreHealth _player 20)
      (Variables|Default|SetUIMessage "The medicine soothes your wounds"))
    (:MysteryLiquid
      (Variables|/Game/Blueprints/Player/BP_Player.BP_Player_C|SetInfectedCounter _player 0)
      (Variables|Default|SetUIMessage "The liquid kills the beasts within you")))
  (CallFunction|UpdateUI))