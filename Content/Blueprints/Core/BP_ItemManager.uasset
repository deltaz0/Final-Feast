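; BP_ItemManager randomly populates the level's BP_Item actors with items when play begins.
; It gathers every BP_Item as a spawn point and despawns all their meshes.
; A single pass then gives each point a one-in-four chance to spawn a random type, with mesh and UI icon looked up from type maps.
; The pass stops once five items spawn, so fewer can appear and earlier array entries are favored.
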(event EventBeginPlay
  (bind _outactors (Actor|GetAllActorsOfClass "/Game/Blueprints/Items/BP_Item.BP_Item_C"))
  (Variables|Default|SetItemSpawns _outactors)
  (CallFunction|InitializeItems))

(fn ConstructionScript)

(fn InitializeItems
  (bind _itemtypes (Variables|Default|GetItemTypes))
  (bind _outitem (Utilities|Array|Random _itemtypes))
  (for _array_element (Variables|Default|GetItemSpawns)
    (Default|DespawnMesh _array_element))
  (bind _array_element_2 (Utilities|Array|ForEachLoopwithBreak (Variables|Default|GetItemSpawns) :!label _label)
    (:LoopBody
      (if (< (Math|Random|RandomInteger 100) 25)
        (Default|SpawnItem _array_element_2 (.Value (Utilities|Map|Find (Variables|Default|GetTypeMeshMap) _outitem)) (.Value (Utilities|Map|Find (Variables|Default|GetTypeIconMap) _outitem)) _outitem)
        (bind _result (Math|Integer|IncrementInt (LocalVariables|GetSpawnCount))
          (:%20%20
            (if (>= _result 5)
              (goto _label Break))))))))