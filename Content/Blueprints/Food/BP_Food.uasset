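; BP_Food is a food actor that the player can hover over and click with the cursor.
; Cursor enter and exit events toggle a hover flag, and Tick spins the actor by a fixed step per frame while it is set.
; A click calls the OnFoodInteraction dispatcher, passing itself.
; Setter functions assign its attribute and static mesh, while Interact and DespawnFood are empty.
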(event Custom|DespawnFood)

(event EventBeginPlay)

(event EventInteract)

(event MouseInput|EventActorOnClicked
  (params (ButtonPressed :type Key%20Structure :default "None"))
  (Default|CallOnFoodInteraction self))

(event MouseInput|EventActorBeginCursorOver
  (Variables|Default|SetIsHovered true))

(event MouseInput|EventActorEndCursorOver
  (Variables|Default|SetIsHovered false))

(event EventTick
  (params (DeltaSeconds :type Float%20%28single-precision%29))
  (if (Variables|Default|GetIsHovered)
    (Transformation|AddActorLocalRotation "0.000000,1.500000,0.000000" false false)))

(fn ConstructionScript)

(fn SetAttribute
  (params (Attribute :type FoodAttribute%20Enum :default "NewEnumerator0"))
  (Variables|Default|SetAttribute Attribute))

(fn SetMesh
  (params (Mesh :type Static%20Mesh%20Object%20Reference))
  (Components|StaticMesh|SetStaticMesh (Variables|Default|GetStaticMesh) Mesh))